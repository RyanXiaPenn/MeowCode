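; CompleteFireBP is a spreadable fire actor driven by a Temperature value that controls ignition, particles, sound and a one-time scorch decal.
; Each tick, burning fires heat up and any instance can randomly gain heat from burning overlapping neighbours, igniting past a threshold.
; A delay loop damages overlapping actors while burning.
; Damage received by a burning fire lowers its temperature, extinguishing it at zero.
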(event `SpawnScorchDecal`
  (if (and (not (`self.HasScorchDecal`)) (>= (`self.Temperature`) 800))
    (`GameplayStatics.SpawnDecalAtLocation` "/Game/Materials/Scorch_mat.Scorch_mat" (100.0 100.0 100.0) (`self.K2_GetActorLocation`))
    (set `self.HasScorchDecal` true)))

(event `self.ReceiveBeginPlay`
  (`self.FireOnChanged`))

(event `self.ReceiveTick`
  (params (DeltaSeconds :type "Float (single-precision)"))
  (`self.FireSpawn`)
  (`self.SpawnScorchDecal`)
  (if (>= (`self.Temperature`) 600)
    (set `self.FireOn` true)
    (`self.FireOnChanged`)))

(event `FireSpawn`
  (if (`self.FireOn`)
    (if (< (`self.Temperature`) 1000)
      (set `self.Temperature` (+ (`self.Temperature`) 1))
      (for _array_element (`self.GetOverlappingActors` "CompleteFireBP_C") :!label _label
        (bind _ascomplete_fire_bp (cast `/Game/CompleteFireBP` _array_element))
        (if (and (> (`KismetMathLibrary.RandomInteger` 10) 6) (`/Game/CompleteFireBP.FireOn` _ascomplete_fire_bp))
          (if (< (`self.Temperature`) 1000)
            (set `self.Temperature` (+ (`self.Temperature`) 1))))))
    (else
      (goto _label))))

(event `FireOnChanged`
  (bind _fireon (`self.FireOn`))
  (`SceneComponent.SetVisibility` (`self.ParticleSystem`) _fireon false)
  (`ActorComponent.SetActive` (`self.FireSound`) _fireon false))

(event `self.ReceiveActorEndOverlap`
  (params (OtherActor :type "Actor Object Reference"))
  (set `self.StillOverlapping` false))

(event `self.ReceiveActorBeginOverlap`
  (params (OtherActor :type "Actor Object Reference"))
  (set `self.StillOverlapping` true)
  (if (and (`self.FireOn`) (`self.StillOverlapping`)) :!label _label_2
    (`GameplayStatics.ApplyDamage` OtherActor 0.04 :!label _label_3)
    (if (and (`self.FireOn`) (`self.StillOverlapping`))
      (`KismetSystemLibrary.Delay` 0.2)
      (goto _label_3))
    (else
      (`KismetSystemLibrary.Delay` 0.2)
      (goto _label_2))))

(event `self.ReceiveAnyDamage`
  (params (Damage :type "Float (single-precision)") (DamageType :type "DamageType Object Reference") (InstigatedBy :type "Controller Object Reference") (DamageCauser :type "Actor Object Reference"))
  (if (`self.FireOn`)
    (bind _output_get (set `self.Temperature` (- (`self.Temperature`) (`KismetMathLibrary.FTrunc` Damage))))
    (set `self.FireOn` (not (<= _output_get 0)))
    (`self.FireOnChanged`)))

(fn `UserConstructionScript`)