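; Pickup actor that refills the fire extinguisher ammo of the FireFighter character.
; On overlap it casts to FireFighter and adds a fixed amount to AmmoForExtinguisher, capped at full.
; It then prints the new value, plays a pickup sound and destroys itself.
; An unconnected older branch targeting FPCharactorBP remains in the graph and never runs.
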(event `self.ReceiveActorBeginOverlap`
  (params (OtherActor :type "Actor Object Reference"))
  (bind _asfire_fighter (cast `/Game/FireFighter` OtherActor))
  (bind _returnvalue (+ (`/Game/FireFighter.AmmoForExtinguisher` _asfire_fighter) 0.2))
  (if (>= _returnvalue 1.0)
    (bind _output_get (set `/Game/FireFighter.AmmoForExtinguisher` 1.0 _asfire_fighter))
    (`KismetSystemLibrary.PrintString` (`KismetStringLibrary.Conv_DoubleToString` _output_get))
    (`GameplayStatics.PlaySound2D` "/Game/Audio/SteamAmmoPickUp.SteamAmmoPickUp" 1.0 1.0 0.0 null null)
    (`self.K2_DestroyActor`)
    (else
      (bind _output_get_2 (set `/Game/FireFighter.AmmoForExtinguisher` _returnvalue _asfire_fighter))
      (`KismetSystemLibrary.PrintString` (`KismetStringLibrary.Conv_DoubleToString` _output_get_2))
      (`GameplayStatics.PlaySound2D` "/Game/Audio/SteamAmmoPickUp.SteamAmmoPickUp" 1.0 1.0 0.0 null null)
      (`self.K2_DestroyActor`))))

(fn `UserConstructionScript`)