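; Resizable fire grid actor that spawns a field of CompleteFireBP cells and starts fires among them at BeginPlay.
; Nested loops lay out GridSizeX by GridSizeY cells at GridSpacer intervals from its location, slightly raised and scaled up.
; For each of NumStartingFires, it gathers all CompleteFireBP actors in the level, raises a random one's Temperature and calls FireOnChanged on a separately randomized pick, so the two can differ.
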(event `self.ReceiveBeginPlay`
  (for _index (range (`self.gridSizeX`))
    (for _index_2 (range (`self.gridSizeY`))
      (`|SpawnActorFromClass` "/Game/CompleteFireBP.CompleteFireBP_C" (`KismetMathLibrary.MakeTransform` (`KismetMathLibrary.MakeVector` (+ (* (`KismetMathLibrary.Conv_IntToDouble` _index) (`self.gridSpacer`)) (.x (`self.K2_GetActorLocation`))) (+ (* (`KismetMathLibrary.Conv_IntToDouble` _index_2) (`self.gridSpacer`)) (.y (`self.K2_GetActorLocation`))) (+ (.z (`self.K2_GetActorLocation`)) 2.0)) (struct) (2.0 2.0 2.0)) "AlwaysSpawn" "OverrideRootScale" null null)))
  (for _ (range (`self.numStartingFires`))
    (bind _outactors (`GameplayStatics.GetAllActorsOfClass` "/Game/CompleteFireBP.CompleteFireBP_C"))
    (bind _output (`|GetArrayItem` _outactors (`KismetMathLibrary.RandomInteger` (`KismetArrayLibrary.Array_Length` _outactors))))
    (set `/Game/CompleteFireBP.Temperature` 600 _output)
    (`/Game/CompleteFireBP.FireOnChanged` _output)))

(fn `UserConstructionScript`)