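; First-person player character Blueprint that manages health and the game's HUD, pause, game-over and win screens.
; BeginPlay creates all four widgets, and the Pause input toggles between HUD and pause menu along with game pause.
; Damage passes through a DoOnce with delayed reset, giving brief invulnerability while a tint flag flashes.
; Zero health or the win event shows its end screen, pauses and switches to UI-only mouse input.
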(event `self.ReceiveBeginPlay`
  (bind _returnvalue (`|CreateWidget` "/Game/MainHUD.MainHUD_C"))
  (bind _output_get (set `self.MainHUDReference` _returnvalue))
  (`UserWidget.AddToViewport` _output_get 0)
  (bind _returnvalue_2 (`|CreateWidget` "/Game/PauseMenu.PauseMenu_C"))
  (set `self.PauseMenuReference` _returnvalue_2)
  (bind _returnvalue_3 (`|CreateWidget` "/Game/GameOverMenu.GameOverMenu_C"))
  (set `self.GameOverMenuReference` _returnvalue_3)
  (bind _returnvalue_4 (`|CreateWidget` "/Game/WinScreenMenu.WinScreenMenu_C"))
  (set `self.WinScreenMenuReference` _returnvalue_4))

(event `EventGameOver`
  (bind _returnvalue (`GameplayStatics.GetPlayerController` 0))
  (bind _gameovermenureference (`self.GameOverMenuReference`))
  (`Widget.RemoveFromParent` (`self.MainHUDReference`))
  (`UserWidget.AddToViewport` _gameovermenureference 0)
  (`WidgetBlueprintLibrary.SetInputMode_UIOnlyEx` _returnvalue _gameovermenureference)
  (set `PlayerController.bShowMouseCursor` true _returnvalue)
  (`GameplayStatics.SetGamePaused` true))

(event `InputAction|Pause` :paused true
  (params (Key :type "Key Structure"))
  (bind _mainhudreference (`self.MainHUDReference`))
  (bind _pausemenureference (`self.PauseMenuReference`))
  (:`Pressed`
    (if (`GameplayStatics.IsGamePaused`)
      (`Widget.RemoveFromParent` _pausemenureference)
      (`UserWidget.AddToViewport` _mainhudreference 0)
      (`GameplayStatics.SetGamePaused` false)
      (else
        (`Widget.RemoveFromParent` _mainhudreference)
        (`UserWidget.AddToViewport` _pausemenureference 0)
        (`GameplayStatics.SetGamePaused` true)))))

(event `self.ReceiveAnyDamage`
  (params (Damage :type "Float (single-precision)") (DamageType :type "DamageType Object Reference") (InstigatedBy :type "Controller Object Reference") (DamageCauser :type "Actor Object Reference"))
  (`/Engine/EditorBlueprintResources/StandardMacros.DoOnce` false :!label _label
    (:`Completed`
      (bind _output_get (set `self.Health` (- (`self.Health`) Damage)))
      (if (<= _output_get 0.0)
        (`self.EventGameOver`)
        (else
          (set `self.ShowDamageTint` true)
          (`KismetSystemLibrary.Delay` 0.2)
          (set `self.ShowDamageTint` false)
          (`KismetSystemLibrary.Delay` 0.2)
          (goto _label :!via `Reset`))))))

(event `EventWinGame`
  (bind _returnvalue (`GameplayStatics.GetPlayerController` 0))
  (bind _winscreenmenureference (`self.WinScreenMenuReference`))
  (`Widget.RemoveFromParent` (`self.MainHUDReference`))
  (`UserWidget.AddToViewport` _winscreenmenureference 0)
  (`WidgetBlueprintLibrary.SetInputMode_UIOnlyEx` _returnvalue _winscreenmenureference)
  (set `PlayerController.bShowMouseCursor` true _returnvalue)
  (`GameplayStatics.SetGamePaused` true))

(fn `UserConstructionScript`
  (`parent.UserConstructionScript`))