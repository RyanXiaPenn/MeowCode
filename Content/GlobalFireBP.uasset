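; GlobalFireBP seeds the fire system by building a grid of CompleteFireBP actors when play begins.
; Nested loops spawn the scaled cells at evenly spaced positions on a fixed-height plane.
; It then repeatedly raises a random cell's Temperature and calls FireOnChanged on a random cell.
; Those two random picks are evaluated separately, so they can land on different cells.
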(event `self.ReceiveBeginPlay`
  (for _index (range 19)
    (for _index_2 (range 22)
      (`|SpawnActorFromClass` "/Game/CompleteFireBP.CompleteFireBP_C" (`KismetMathLibrary.MakeTransform` (`KismetMathLibrary.MakeVector` (- (* (`KismetMathLibrary.Conv_IntToDouble` _index) 119.0) 935.0) (+ (* (`KismetMathLibrary.Conv_IntToDouble` _index_2) 118.0) -920.0) 298.0) (struct) (2.0 2.0 2.0)) "AlwaysSpawn" "OverrideRootScale" null null)))
  (for _ (range 10)
    (bind _outactors (`GameplayStatics.GetAllActorsOfClass` "/Game/CompleteFireBP.CompleteFireBP_C"))
    (bind _output (`|GetArrayItem` _outactors (`KismetMathLibrary.RandomInteger` (`KismetArrayLibrary.Array_Length` _outactors))))
    (set `/Game/CompleteFireBP.Temperature` 600 _output)
    (`/Game/CompleteFireBP.FireOnChanged` _output)))

(fn `UserConstructionScript`)